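; BP_BoardSpace is a board tile actor that steers player avatars moving across the game board.
; It tracks whether something overlaps it through begin and end overlap events, exposed via CheckOverlap.
; MoreToMove casts the given actor to BP_PlayerAvatar and passes the space's stored Direction to its MoveTest, printing a message if the cast fails.
; GetBoardType is an empty stub.
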(event `self.ReceiveActorBeginOverlap`
  (params (OtherActor :type "Actor Object Reference"))
  (set `self.Overlapped` true))

(event `self.ReceiveActorEndOverlap`
  (params (OtherActor :type "Actor Object Reference"))
  (set `self.Overlapped` false))

(event `MoreToMove`
  (params (`Actor Overlapping` :type "Actor Object Reference"))
  (bind _asbp_player_avatar (cast `/Game/Blueprints/Character/BP_PlayerAvatar` `Actor Overlapping`)
    (:`then`
      (bind _direction (`self.GetDirection`))
      (`/Game/Blueprints/Character/BP_PlayerAvatar.MoveTest` _asbp_player_avatar _direction))
    (:`CastFailed`
      (`KismetSystemLibrary.PrintString` "Overlap was not PlayerAvatar"))))

(fn `CheckOverlap`
  (returns (Overlapped :type Boolean))
  (bind _overlapped (`self.Overlapped`))
  (if _overlapped
    (return _overlapped)
    (else
      (return _overlapped))))

(fn `GetBoardType`)

(fn `GetDirection`
  (returns (Direction :type "EDirection Enum"))
  (return (`self.Direction`)))

(fn `UserConstructionScript`)